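; Game instance that tracks progression from reported enemy, object and location events.
; ReportEvent accumulates amounts in a counter map keyed by "Type:TargetID", then runs EvaluateStep.
; EvaluateStep scans DT_ProgressionStep, checking counts for enemies and objects and key presence for locations, then broadcasts OnProgressionEvent and records each completed step to prevent repeats.
; Camera registration and switching events are empty stubs.
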(event `/Game/ThirdPerson/Camera/BPI_CameraManager.ReturnToPlayer`)

(event `/Game/ThirdPerson/Camera/BPI_CameraManager.SwitchToCamera`)

(event `/Game/ThirdPerson/Camera/BPI_CameraManager.RegisterCamera`)

(event `/Game/ThirdPerson/Camera/BPI_CameraManager.SetCameraManager`)

(fn `EvaluateStep`
  (bind _outrownames (`DataTableFunctionLibrary.GetDataTableRowNames` "/Game/ThirdPerson/Progresion/DT_ProgressionStep.DT_ProgressionStep"))
  (for _array_element _outrownames
    (bind _returnvalue (`|GetDataTableRow` "/Game/ThirdPerson/Progresion/DT_ProgressionStep.DT_ProgressionStep" _array_element)
      (:`then`
        (bind (_stepid _targetid _conditiontype _requertamount _actiontarget) (break `/Game/ThirdPerson/Progresion/S_ProgressionStep` _returnvalue))
        (if (not (`BlueprintSetLibrary.Set_Contains` (`self.CompletedStep`) _stepid))
          (switch `/Game/ThirdPerson/Progresion/E_ConditionType` _conditiontype
            (:`NewEnumerator0`
              (bind _returnvalue_2 (`KismetStringLibrary.Conv_StringToName` (`KismetStringLibrary.Concat_StrStr` (`|GetEnumeratorNameAsString` _conditiontype) ":" (`KismetStringLibrary.Conv_NameToString` _targetid))))
              (bind _value (`self.GetCounter` _returnvalue_2 :!label _label))
              (if (>= _value _requertamount)
                (`self.OnProgressionEvent` _stepid _actiontarget :!label _label_2)
                (`BlueprintSetLibrary.Set_Add` (`self.CompletedStep`) _stepid)))
            (:`NewEnumerator1`
              (goto _label))
            (:`NewEnumerator2`
              (bind _value_2 (`self.GetFlag` _returnvalue_2))
              (if _value_2
                (goto _label_2)))))))))

(fn `GetCounter`
  (params (Key :type Name))
  (returns (Value :type Integer))
  (return (`BlueprintMapLibrary.Map_Find` (`self.ProgresionCounters`) Key)))

(fn `GetFlag`
  (params (Key :type Name))
  (returns (Value :type Boolean))
  (return (`.ReturnValue` (`BlueprintMapLibrary.Map_Find` (`self.ProgresionCounters`) Key))))

(fn `ReportEvent`
  (params (Type :type "/Game/ThirdPerson/Progresion/E_ConditionType Enum" :default "NewEnumerator0") (TargetID :type Name) (Amount :type Integer))
  (bind _amount (`local.Amount`))
  (bind _progresioncounters (`self.ProgresionCounters`))
  (bind _returnvalue (`KismetStringLibrary.Conv_StringToName` (`KismetStringLibrary.Concat_StrStr` (`|GetEnumeratorNameAsString` Type) ":" (`KismetStringLibrary.Conv_NameToString` TargetID))))
  ; Reportar Eventos, este evento tiene un tip, si es enemigo u objeto
  ;; Si es un nuevo enemigo lo pone y si no lo es suma los que ya haya derrotado
  (if true
    (`BlueprintMapLibrary.Map_Add` _progresioncounters _returnvalue (+ (`BlueprintMapLibrary.Map_Find` _progresioncounters _returnvalue) _amount))
    (else
      (`BlueprintMapLibrary.Map_Add` _progresioncounters _returnvalue _amount)))
  (`self.EvaluateStep`))
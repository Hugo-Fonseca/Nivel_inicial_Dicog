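; BP_Projectile_TokPok is a projectile actor that deals fixed damage to what it hits.
; When its collision component hits any actor other than its owner, it fires OnProjectileHit with the actor and hit result.
; It then sends a damage info struct to that actor's BPC_DamageSystem component through a TakeDamage message and destroys itself.
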(event `self.ProjectileCollision.OnComponentHit`
  (params (HitComponent :type "PrimitiveComponent Object Reference") (OtherActor :type "Actor Object Reference") (OtherComp :type "PrimitiveComponent Object Reference") (NormalImpulse :type "Vector Structure") (Hit :type "HitResult Structure (by ref)"))
  (if (not (== OtherActor (`self.GetOwner`)))
    (`self.OnProjectileHit` OtherActor Hit)
    (message `/Game/TestGame/DamageSystem/BPI_Damageable.TakeDamage` (`self.GetComponentByClass` OtherActor "/Game/TestGame/Blueprints/Components/BPC_DamageSystem.BPC_DamageSystem_C") (make `/Game/TestGame/DamageSystem/S_DamageInfo` 25.0 "NewEnumerator2"))
    (`self.K2_DestroyActor`)))

(fn `UserConstructionScript`
  (`parent.UserConstructionScript`))
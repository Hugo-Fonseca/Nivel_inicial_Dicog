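; Configurable projectile actor that flies at an optional target, reports what it hits through OnProjectileHit, then destroys itself.
; The construction script applies speed and gravity to ProjectileMovement, plus homing on the target's root component when enabled.
; BeginPlay ignores the owner for collision, aims velocity at any valid target and starts a lifespan timer.
; Hits on anything except the owner trigger the callback and destruction.
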(event `self.ReceiveBeginPlay`
  (`PrimitiveComponent.IgnoreActorWhenMoving` (`self.ProjectileCollision`) (`self.GetOwner`) true)
  (`self.Target`
    (:`then`
      (`self.Rotate To Target`))
    (:`else`
      _))
  (`KismetSystemLibrary.K2_SetTimerDelegate` (delegate `Destroy Projectile`) (`self.ProjectileLifespan`)))

(event `Destroy Projectile`
  (`self.K2_DestroyActor`))

(event `Rotate To Target`
  (set `MovementComponent.Velocity` (* (`KismetMathLibrary.GetDirectionUnitVector` (`self.K2_GetActorLocation`) (`self.K2_GetActorLocation` (`self.Target`))) (`self.ProjectileSpeed`)) (`self.ProjectileMovement`)))

(event `self.ProjectileCollision.OnComponentHit`
  (params (HitComponent :type "PrimitiveComponent Object Reference") (OtherActor :type "Actor Object Reference") (OtherComp :type "PrimitiveComponent Object Reference") (NormalImpulse :type "Vector Structure") (Hit :type "HitResult Structure (by ref)"))
  (if (not (== OtherActor (`self.GetOwner`)))
    (`self.OnProjectileHit` OtherActor Hit)
    (`self.K2_DestroyActor`)))

(fn `UserConstructionScript`
  (bind _projectilemovement (`self.ProjectileMovement`))
  (bind _ishoming (`self.IsHoming`))
  (bind _output_get (set `ProjectileMovementComponent.InitialSpeed` (`self.ProjectileSpeed`) _projectilemovement))
  (set `ProjectileMovementComponent.MaxSpeed` _output_get _projectilemovement)
  (set `ProjectileMovementComponent.ProjectileGravityScale` (`self.ProjectileGravity`) _projectilemovement)
  (bind _target (`self.Target`)
    (:`then`
      (if _ishoming
        (set `ProjectileMovementComponent.bIsHomingProjectile` _ishoming _projectilemovement)
        (set `ProjectileMovementComponent.HomingAccelerationMagnitude` (`self.HomingSpeed`) _projectilemovement)
        (set `ProjectileMovementComponent.HomingTargetComponent` (`Actor.RootComponent` _target) _projectilemovement)))
    (:`else`)))
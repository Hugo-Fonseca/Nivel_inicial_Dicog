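; Health component that handles healing and damage, tracking death, invincibility, blocking and interruption, and firing heal, block, damage and death events.
; TakeDamage only proceeds for a guarding BP_Player owner, then uses a CanBeDamaged macro to block, apply or ignore the hit.
; The guard damage multiplier is wired but unused, as its select always picks the raw amount.
; Non-lethal hits fire the damage event only when interruptible or force-interrupting.
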(fn `Heal`
  (params (Amount :type "Float (double-precision)"))
  (returns (`New Health` :type "Float (double-precision)"))
  (if (not (`self.IsDead`))
    (bind _output_get (set `self.Health` (`KismetMathLibrary.FClamp` (+ Amount (`self.Health`)) 0.0 (`self.MaxHealth`))))
    (`self.OnHeal`)
    (return _output_get)))

(fn `TakeDamage`
  (params (DamageInfo :type "/Game/TestGame/DamageSystem/S_DamageInfo Structure"))
  (returns (`Was Damaged` :type Boolean))
  (bind (_amount _damagetype _damageresponse _shoulddamageinvincible _canbeblocked _canbeparried _shouldforceinterrupt) (break `/Game/TestGame/DamageSystem/S_DamageInfo` DamageInfo))
  (bind _asbp_player (cast `/Game/TestGame/Blueprints/BP_Player` (`self.GetOwner`)))
  (if (`/Game/TestGame/Blueprints/BP_Player.ISGuarding` _asbp_player)
    (`self.CanBeDamaged` _shoulddamageinvincible _canbeblocked
      (:`BlockDamage`
        (`KismetSystemLibrary.PrintString` "Blocked")
        (`self.OnBlocked` _canbeparried)
        (return false))
      (:`DoDamage`
        (bind _output_get (set `self.Health` (- (`self.Health`) (`KismetMathLibrary.SelectFloat` (* _amount (`/Game/TestGame/Blueprints/BP_Player.GuardDamageMultipler` _asbp_player)) _amount))))
        (if (<= _output_get 0.0)
          (set `self.IsDead` true)
          (`self.OnDeath`)
          (return true)
          (elif (or (`self.IsInterruptible`) _shouldforceinterrupt)
            (`self.OnDamage` _damageresponse)
            (return true))))
      (:`NoDamage`
        (`KismetSystemLibrary.PrintString` "No Damage")
        (return false)))))
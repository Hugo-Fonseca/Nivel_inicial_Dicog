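; Lock-on targeting component that toggles a lock onto BPI_Lockable actors around its owning Character.
; A debug-drawn sphere trace gathers candidates, then selection keeps the last with a visibility-trace hit and camera-forward dot product above Comparetarget, which never updates.
; Locking shows the target's widget and disables movement-driven rotation; Tick then turns character yaw and control rotation toward the target.
; Unlocking hides the widget and re-enables movement rotation.
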(event `self.ReceiveBeginPlay`
  (bind _ascharacter (cast `Character` (`self.GetOwner`)))
  (set `self.Character Ref` _ascharacter)
  (set `self.Camera Ref` (`Actor.GetComponentByClass` (`self.Character Ref`) "/Script/Engine.CameraComponent")))

(event `Lock On To target`
  (bind _targetingactor (`self.Find Actor To Lock On To`))
  (bind _closettarget (`self.Find Closet Target` _targetingactor))
  (`/Engine/EditorBlueprintResources/StandardMacros.IsValid` _closettarget
    (:`Is Valid`
      (bind _output_get (set `self.LockOnActor` _closettarget))
      (message `/Game/TestGame/Blueprints/BPI_Interface/BPI_TargetingInterface.DisplayLockedOnWidget` _output_get true)
      (`self.Orient Camera`)
      (set `self.LockedOn?` true))))

(event `Stop Lock On`
  (bind _lockonactor (`self.LockOnActor`))
  (`/Engine/EditorBlueprintResources/StandardMacros.IsValid` _lockonactor
    (:`Is Valid`
      (message `/Game/TestGame/Blueprints/BPI_Interface/BPI_TargetingInterface.DisplayLockedOnWidget` _lockonactor false)
      (set `self.LockOnActor` null)
      (set `self.LockedOn?` false)
      (`self.OrientMovement`))))

(event `Toggle Lock On`
  (if (`self.LockedOn?`)
    (`self.Stop Lock On`)
    (else
      (`self.Lock On To target`))))

(event `Orient Camera`
  (bind _charactermovement (`Character.CharacterMovement` (`self.Character Ref`)))
  (set `CharacterMovementComponent.bOrientRotationToMovement` false _charactermovement)
  (set `CharacterMovementComponent.bUseControllerDesiredRotation` false _charactermovement))

(event `OrientMovement`
  (bind _charactermovement (`Character.CharacterMovement` (`self.Character Ref`)))
  (set `CharacterMovementComponent.bOrientRotationToMovement` true _charactermovement)
  (set `CharacterMovementComponent.bUseControllerDesiredRotation` true _charactermovement))

(event `self.ReceiveTick`
  (params (DeltaSeconds :type "Float (single-precision)"))
  (if (`self.LockedOn?`)
    (`self.Face Locked On Actor`)))

(fn `Check How Close Target Is`
  (params (Target :type "Actor Object Reference"))
  (returns (ReturnValue :type "Float (double-precision)"))
  (return (`KismetMathLibrary.Dot_VectorVector` (`SceneComponent.GetForwardVector` (`self.Camera Ref`)) (`KismetMathLibrary.Conv_RotatorToVector` (`KismetMathLibrary.FindLookAtRotation` (`Actor.K2_GetActorLocation` (`self.Character Ref`)) (`Actor.K2_GetActorLocation` Target))))))

(fn `Face Locked On Actor`
  (bind _character_ref (`self.Character Ref`))
  (bind _returnvalue (`Pawn.GetController` (`self.Character Ref`)))
  (bind _returnvalue_2 (`Controller.GetControlRotation` _returnvalue))
  (bind _yaw (.yaw (`KismetMathLibrary.RInterpTo_Constant` _returnvalue_2 (`KismetMathLibrary.FindLookAtRotation` (`Actor.K2_GetActorLocation` _character_ref) (- (`Actor.K2_GetActorLocation` (`self.LockOnActor`)) (0.0 0.0 90.0))) (`GameplayStatics.GetWorldDeltaSeconds`) (`self.Interp Speed`))))
  (`Actor.K2_SetActorRotation` _character_ref (`KismetMathLibrary.MakeRotator` 0.0 0.0 _yaw) false)
  (`Controller.SetControlRotation` _returnvalue (`KismetMathLibrary.MakeRotator` (.roll _returnvalue_2) (.pitch (`KismetMathLibrary.RInterpTo_Constant` _returnvalue_2 (`KismetMathLibrary.FindLookAtRotation` (`Actor.K2_GetActorLocation` _character_ref) (- (`Actor.K2_GetActorLocation` (`self.LockOnActor`)) (0.0 0.0 90.0))) (`GameplayStatics.GetWorldDeltaSeconds`) (`self.Interp Speed`))) _yaw)))

(fn `Find Actor To Lock On To`
  (returns (TargetingActor :type "Array of Actor Object Reference"))
  (locals (PotentialTargetingActor :type "Array of Actor Object Reference"))
  (bind _returnvalue (`Actor.K2_GetActorLocation` (`self.Character Ref`)))
  (bind (_outhits _returnvalue_2) (`KismetSystemLibrary.SphereTraceMultiForObjects` _returnvalue _returnvalue (`self.Radius`) (`|MakeArray` "ObjectTypeQuery10" "ObjectTypeQuery3" :!type "EObjectTypeQuery Enum") false (`|MakeArray` (`self.GetOwner`)) "ForDuration" true (struct :`R` 1.0 :`A` 1.0) (struct :`G` 1.0 :`A` 1.0) 1.0))
  (for _array_element _outhits
    (bind (_bblockinghit _binitialoverlap _time _distance _location _impactpoint _normal _impactnormal _physmat _hitactor) (`GameplayStatics.BreakHitResult` _array_element))
    (if (and _returnvalue_2 (`KismetSystemLibrary.DoesImplementInterface` _hitactor "/Game/TestGame/WidgetManager/BPI_Lockable.BPI_Lockable_C"))
      (`KismetArrayLibrary.Array_Add` (`local.PotentialTargetingActor`) _hitactor)))
  (return (`local.PotentialTargetingActor`)))

(fn `Find Closet Target`
  (params (Actors :type "Array of Actor Object Reference"))
  (returns (closettarget :type "Actor Object Reference"))
  (locals (Comparetarget :type "Float (double-precision)") (closesttarget :type "Actor Object Reference"))
  (bind _comparetarget (`local.Comparetarget`))
  (for _array_element Actors
    (bind (_outhit _returnvalue) (`KismetSystemLibrary.LineTraceSingle` :`Start` (`SceneComponent.K2_GetComponentLocation` (`self.Camera Ref`)) :`End` (`Actor.K2_GetActorLocation` _array_element) :`TraceChannel` "TraceTypeQuery1" :`DrawDebugType` "ForDuration"))
    (if _returnvalue
      (`/Engine/EditorBlueprintResources/StandardMacros.CompareFloat` (`self.Check How Close Target Is` _array_element) _comparetarget
        (:`>`
          (set `local.Comparetarget` _comparetarget)
          (set `local.closesttarget` _array_element)))))
  (return (`local.closesttarget`)))
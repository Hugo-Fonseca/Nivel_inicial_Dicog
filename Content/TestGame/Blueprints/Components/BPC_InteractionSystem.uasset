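; Actor component that lets its owning character detect and interact with nearby actors implementing BPI_Interactable.
; Capsule overlaps maintain an in-range list whose most recent entry is active and gets a screen-space prompt widget at its location.
; Press, Hold and Tap interactions are driven through interface queries, showing progress on the widget.
; On completion the owner turns to face the target and sends it an Interact message.
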(event `self.ReceiveBeginPlay`
  (bind _ascharacter (cast `Character` (`self.GetOwner`)))
  (bind _capsulecomponent (`Character.CapsuleComponent` _ascharacter))
  (add `PrimitiveComponent.OnComponentBeginOverlap` _capsulecomponent (`|CreateDelegate` :!event `On Begin Overlap`))
  (add `PrimitiveComponent.OnComponentEndOverlap` _capsulecomponent (`|CreateDelegate` :!event `On End Overlap`))
  (bind _returnvalue (`|AddComponentByClass` :`self` (`self.GetOwner`) :`Class` "/Script/UMG.WidgetComponent" :`bManualAttachment` true))
  (`WidgetComponent.SetWidgetSpace` _returnvalue "Screen")
  (`WidgetComponent.SetDrawSize` _returnvalue (32.0 32.0))
  (set `self.InteractionWidget` _returnvalue))

(event `On Begin Overlap`
  (params (OverlappedComponent :type "PrimitiveComponent Object Reference") (OtherActor :type "Actor Object Reference") (OtherComp :type "PrimitiveComponent Object Reference") (OtherBodyIndex :type Integer) (bFromSweep :type Boolean) (SweepResult :type "HitResult Structure (by ref)"))
  (`self.IsInteractable` OtherActor
    (:`True`
      (`KismetArrayLibrary.Array_AddUnique` (`self.InteractablesInRange`) OtherActor)
      (`self.RenderInteractionWidget` :!label _label))))

(event `On End Overlap`
  (params (OverlappedComponent :type "PrimitiveComponent Object Reference") (OtherActor :type "Actor Object Reference") (OtherComp :type "PrimitiveComponent Object Reference") (OtherBodyIndex :type Integer))
  (`self.IsInteractable` OtherActor
    (:`True`
      (if (== OtherActor (`self.GetActiveInteractable`))
        (set `self.CurrentTapCount` 0))
      (`KismetArrayLibrary.Array_RemoveItem` (`self.InteractablesInRange`) OtherActor)
      (goto _label))))

(event `InteractWithActor`
  (bind _active_interactable (`self.GetActiveInteractable`))
  (bind _returnvalue (`self.GetOwner`))
  (bind (_returnvalue_roll _returnvalue_pitch _returnvalue_yaw) (`KismetMathLibrary.BreakRotator` (`KismetMathLibrary.FindLookAtRotation` (`Actor.K2_GetActorLocation` _returnvalue) (`self.GetActiveInteractableLocation`))))
  (`/Engine/EditorBlueprintResources/StandardMacros.IsValid` _active_interactable
    (:`Is Valid`
      (`Actor.K2_SetActorRotation` _returnvalue (`KismetMathLibrary.MakeRotator` 0.0 0.0 _returnvalue_yaw) false)
      (message `/Game/TestGame/InteractionSystem/BPI_Interactable.Interact` _active_interactable _returnvalue))))

(event `InteractionBegin`
  (bind _active_interactable (`self.GetActiveInteractable`))
  (`/Engine/EditorBlueprintResources/StandardMacros.IsValid` _active_interactable
    (:`Is Valid`
      (bind _interaction_type (message `/Game/TestGame/InteractionSystem/BPI_Interactable.GetInteractionType` _active_interactable))
      (switch `/Game/TestGame/InteractionSystem/E_InteractionType` _interaction_type
        (:`NewEnumerator0`
          (`self.InteractWithActor` :!label _label_2)
          (`self.InteractionOver`))
        (:`NewEnumerator1`
          (add `self.OnInteractPressOngoing` (`|CreateDelegate` :!event `InteractionOngoing`))
          (add `self.OnInteractEnded` (delegate `HoldEnd`)))
        (:`NewEnumerator2`
          (`self.InteractionTapOngoing`))))))

(event `InteractionOver`
  (`/Engine/EditorBlueprintResources/StandardMacros.IsValid` (`self.GetActiveInteractable`)
    (:`Is Valid`
      (`/Game/TestGame/Blueprints/Widgets/WBP_Interaction.SetProgressPercent` (`self.InteractionWidgetRef`) 0.0))))

(event `HoldEnd`
  (`self.InteractionOver`)
  (remove `self.OnInteractEnded` (delegate `HoldEnd`)))

(event `InteractionTapOngoing`
  (bind _currenttapcount (`self.CurrentTapCount`))
  (bind _result (`/Engine/EditorBlueprintResources/StandardMacros.IncrementInt` (`self.CurrentTapCount`))
    (:`  `
      (bind _value (message `/Game/TestGame/InteractionSystem/BPI_Interactable.GetTapCount` (`self.GetActiveInteractable`)))
      (if (<= _value _result)
        (goto _label_2)
        (else
          (bind _interactionwidgetref (`self.InteractionWidgetRef`)
            (:`then`
              (`/Game/TestGame/Blueprints/Widgets/WBP_Interaction.SetProgressPercent` _interactionwidgetref (/ _currenttapcount _value))
              (if (>= _currenttapcount _value)
                (set `self.CurrentTapCount` 0)
                (goto _label_2)))
            (:`else`)))))))

(event `InteractionOngoing` :!signature `self.OnInteractPressOngoing`
  (params (`Elapsed Time` :type "Float (double-precision)"))
  (bind _active_interactable (`self.GetActiveInteractable`))
  (`/Engine/EditorBlueprintResources/StandardMacros.IsValid` _active_interactable
    (:`Is Valid`
      (bind _holdduration (message `/Game/TestGame/InteractionSystem/BPI_Interactable.GetHoldDuration` _active_interactable))
      (bind _interactionwidgetref (`self.InteractionWidgetRef`)
        (:`then`
          (`/Game/TestGame/Blueprints/Widgets/WBP_Interaction.SetProgressPercent` _interactionwidgetref (/ `Elapsed Time` _holdduration)))
        (:`else`
          _))
      (if (>= `Elapsed Time` _holdduration)
        (remove `self.OnInteractPressOngoing` (delegate `InteractionOngoing`))
        (goto _label_2)))))

(fn `GetActiveInteractable`
  (returns (`Active Interactable` :type "Actor Object Reference"))
  (bind _interactablesinrange (`self.InteractablesInRange`))
  (return (`|GetArrayItem` _interactablesinrange (`KismetArrayLibrary.Array_LastIndex` _interactablesinrange))))

(fn `GetActiveInteractableLocation`
  (returns (ReturnValue :type "Vector Structure"))
  (bind _active_interactable (`self.GetActiveInteractable`))
  (bind _location (message `/Game/TestGame/InteractionSystem/BPI_Interactable.GetInteractionLocation` _active_interactable))
  (return (`KismetMathLibrary.SelectVector` (`Actor.K2_GetActorLocation` _active_interactable) _location (`KismetMathLibrary.EqualExactly_VectorVector` _location))))

(fn `RenderInteractionWidget`
  (bind _active_interactable (`self.GetActiveInteractable`))
  (bind _interactionwidget (`self.InteractionWidget`))
  (`/Engine/EditorBlueprintResources/StandardMacros.IsValid` _active_interactable
    (:`Is Valid`
      (bind _interaction_type (message `/Game/TestGame/InteractionSystem/BPI_Interactable.GetInteractionType` _active_interactable))
      (bind _returnvalue (`|GenericCreateObject` (`self.GetOwner`) "/Game/TestGame/Blueprints/Widgets/WBP_Interaction.WBP_Interaction_C" _interaction_type))
      (bind _output_get (set `self.InteractionWidgetRef` _returnvalue))
      (`WidgetComponent.SetWidget` _interactionwidget _output_get)
      (`SceneComponent.K2_SetWorldLocation` _interactionwidget (`self.GetActiveInteractableLocation`) false false))
    (:`Is Not Valid`
      (`WidgetComponent.SetWidget` _interactionwidget null))))
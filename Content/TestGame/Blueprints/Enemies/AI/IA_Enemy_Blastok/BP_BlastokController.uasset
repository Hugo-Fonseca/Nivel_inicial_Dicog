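; AI controller for the Blastok enemy that starts and feeds its behavior tree.
; BeginPlay runs BT_Blastok.
; Every tick it casts the controlled pawn to BP_Enemy_Blastok and copies its player reference and detection flag into the blackboard for the tree to use.
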(event `self.ReceiveBeginPlay`
  (`self.RunBehaviorTree` "/Game/TestGame/Blueprints/Enemies/AI/IA_Enemy_Blastok/BT_Blastok.BT_Blastok"))

(event `self.ReceiveTick`
  (params (DeltaSeconds :type "Float (single-precision)"))
  (bind _returnvalue (`AIBlueprintHelperLibrary.GetBlackboard` null))
  (bind _asbp_enemy_blastok (cast `/Game/TestGame/Blueprints/Enemies/BP_Enemy_Blastok` (`self.K2_GetPawn`)))
  (`BlackboardComponent.SetValueAsObject` _returnvalue (`self.TargetPlayerKey`) (`/Game/TestGame/Blueprints/Enemies/BP_Enemy_Blastok.PlayerReference` _asbp_enemy_blastok))
  (`BlackboardComponent.SetValueAsBool` _returnvalue (`self.detectedKey`) (`/Game/TestGame/Blueprints/Enemies/BP_Enemy_Blastok.IsPlayerDetected` _asbp_enemy_blastok)))

(fn `UserConstructionScript`)
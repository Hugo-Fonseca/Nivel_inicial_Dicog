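; Special door Blueprint that opens in response to game progression events rather than player interaction.
; On BeginPlay it binds to the game instance's progression event, and when the action target matches its TargetID, it switches on the step ID and rotates the door mesh open.
; It implements interaction functions with placeholder returns, but Interact is empty and the old open/close toggle is left disconnected.
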(event `self.ReceiveBeginPlay`
  (add `/Game/TestGame/Games_Instance/BP_GamesInstance.OnProgressionEvent` (`/Game/ThirdPerson/Progresion/BFL_GameInstance.GetMyGameInstance`) (delegate `Desbloquear`)))

(event `Desbloquear`
  (params (StepID :type Name) (ActionTarget :type Name))
  (if (== ActionTarget (`self.TargetID`))
    (switch `name` StepID
      (:`Default`
        (`SceneComponent.K2_SetRelativeRotation` (`self.DoorMesh`) (`KismetMathLibrary.MakeRotator` 0.0 0.0 90.0) false false)))))

(event `self.Interact`
  (params (Interactor :type "Actor Object Reference")))

(fn `GetHoldDuration`
  (returns (HoldDuration :type "Float (double-precision)"))
  (return 0.0))

(fn `GetInteractionLocation`
  (returns (Location :type "Vector Structure"))
  (return (0.0 0.0 0.0)))

(fn `GetInteractionType`
  (returns (`Interaction Type` :type "/Game/TestGame/InteractionSystem/E_InteractionType Enum"))
  (return "NewEnumerator0"))

(fn `GetTapCount`
  (returns (Value :type Integer))
  (return 0))

(fn `UserConstructionScript`)
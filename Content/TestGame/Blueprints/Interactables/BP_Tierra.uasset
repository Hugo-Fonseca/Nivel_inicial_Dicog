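; BP_Tierra is an interactable pickup that grants the player the Earth (Tierra) element or Earth energy.
; On a valid interaction it casts the player character to BP_Player and checks the current element state.
; If Earth is active it sends an energy-add message; otherwise it unlocks Earth, makes it current and sets its starting ability value.
; Both branches print debug text and destroy the pickup.
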(event `self.IsValidInteraction`
  (params (CanInteract :type Boolean))
  (if CanInteract
    (bind _asbp_player (cast `/Game/TestGame/Blueprints/BP_Player` (`GameplayStatics.GetPlayerCharacter` 0))
      (:`then`
        (`KismetSystemLibrary.PrintString` (`KismetSystemLibrary.GetDisplayName` _asbp_player))
        (`KismetSystemLibrary.PrintString` "Cast Ok")
        (if (`|EnumEquality` (`/Game/TestGame/Blueprints/BP_Player.CurrentElementState` _asbp_player) "NewEnumerator3")
          (message `/Game/TestGame/WidgetManager/BPI_ElementPickup.AgregarEnergia` _asbp_player 0.2 "NewEnumerator3")
          (`KismetSystemLibrary.PrintString` "Ya tienes el elemneto Tierra")
          (`self.K2_DestroyActor`)
          (else
            (set `/Game/TestGame/Blueprints/BP_Player.TienePoderTierra` true _asbp_player)
            (set `/Game/TestGame/Blueprints/BP_Player.CurrentElementState` "NewEnumerator3" _asbp_player)
            (set `/Game/TestGame/Blueprints/BP_Player.HabilidadTierra` (+ 0.0 0.2) _asbp_player)
            (`KismetSystemLibrary.PrintString` "Desbloqueado Eleemnto Tierra")
            (`self.K2_DestroyActor`))))
      (:`CastFailed`
        (`KismetSystemLibrary.PrintString` "Cast Fallo")))))

(event `self.StartInteraction`)

(fn `UserConstructionScript`)
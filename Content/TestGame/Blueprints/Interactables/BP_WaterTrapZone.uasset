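; BP_WaterTrapZone is a trap volume that makes water pillars rise at random once the player enters it.
; A TriggerZone overlap by BP_Player sets TrapActive and starts a looping timer with a fixed interval.
; Each timer tick calls RiseWater on a random entry in the WaterPillars array.
; The graph has no logic to stop the timer or clear TrapActive.
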(event `self.TriggerZone.OnComponentBeginOverlap`
  (params (OverlappedComponent :type "PrimitiveComponent Object Reference") (OtherActor :type "Actor Object Reference") (OtherComp :type "PrimitiveComponent Object Reference") (OtherBodyIndex :type Integer) (bFromSweep :type Boolean) (SweepResult :type "HitResult Structure (by ref)"))
  (cast `/Game/TestGame/Blueprints/BP_Player` OtherActor)
  (set `self.TrapActive` true)
  (`KismetSystemLibrary.K2_SetTimerDelegate` (delegate `ActivateRandomPillar`) 2.0 true))

(event `ActivateRandomPillar`
  (`/Game/TestGame/Blueprints/Interactables/BP_WaterPillar1.RiseWater` (`|GetArrayItem` (`self.WaterPillars`) (`KismetMathLibrary.RandomIntegerInRange` 0 (- (`KismetArrayLibrary.Array_Length` (`self.WaterPillars`)) 1)))))

(fn `UserConstructionScript`)
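; BP_WaterPillar1 is a rising pillar hazard that damages BP_Player through its BPCDamageSystem on DamageBox overlap.
; BeginPlay sinks the mesh by Height; RiseWater plays a timeline over a fixed offset, enables the box, waits, reverses, waits hidden, then repeats.
; Nothing in this graph starts RiseWater, and the box's collision is never disabled again.
; Timeline and debug names refer to fire despite the water name.
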(event `RiseWater`
  (set `self.IsGoingUp` true)
  (bind (_direction _newtrack_0) (`Timeline|TL_FireRise` :!label _label)
    (:`Update`
      (`SceneComponent.K2_SetRelativeLocation` (`self.PillarMesh`) (`KismetMathLibrary.VLerp` (0.0 0.0 -500.0) (0.0 0.0 0.0) _newtrack_0) false false))
    (:`Finished`
      (if (`self.IsGoingUp`)
        (`PrimitiveComponent.SetCollisionEnabled` (`self.DamageBox`) "QueryOnly")
        (`KismetSystemLibrary.Delay` (`self.ActiveTime`))
        (set `self.IsGoingUp` false)
        (goto _label :!via `Reverse`)
        (else
          (`KismetSystemLibrary.Delay` (`self.HiddenTime`))
          (`self.RiseWater`))))))

(event `self.ReceiveBeginPlay`
  (`SceneComponent.K2_SetRelativeLocation` (`self.PillarMesh`) (`KismetMathLibrary.MakeVector` 0.0 0.0 (* (`self.Height`) -1.0)) false false))

(event `self.DamageBox.OnComponentBeginOverlap`
  (params (OverlappedComponent :type "PrimitiveComponent Object Reference") (OtherActor :type "Actor Object Reference") (OtherComp :type "PrimitiveComponent Object Reference") (OtherBodyIndex :type Integer) (bFromSweep :type Boolean) (SweepResult :type "HitResult Structure (by ref)"))
  (bind _asbp_player (cast `/Game/TestGame/Blueprints/BP_Player` OtherActor))
  (`/Game/TestGame/Blueprints/Components/BPC_DamageSystem.TakeDamage` (`/Game/TestGame/Blueprints/BP_Player.BPC_DamageSystem` _asbp_player) (make `/Game/TestGame/DamageSystem/S_DamageInfo` 10.0 "NewEnumerator4"))
  (`KismetSystemLibrary.PrintString` "Quemado pilar"))

(fn `UserConstructionScript`)
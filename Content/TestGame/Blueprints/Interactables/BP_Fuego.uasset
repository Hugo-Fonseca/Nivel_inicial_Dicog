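; BP_Fuego is an interactable fire-element pickup that unlocks or recharges the player's fire power.
; On a valid interaction it casts to BP_Player, then adds energy if fire is the current element, otherwise grants fire as the current element with starting charge, and destroys itself.
; It binds SpawnearFuego to the game instance's progression event, filtered by TargetID, though the step switch has no visible actions.
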(event `self.ReceiveBeginPlay`
  (add `/Game/TestGame/Games_Instance/BP_GamesInstance.OnProgressionEvent` (`/Game/ThirdPerson/Progresion/BFL_GameInstance.GetMyGameInstance`) (delegate `SpawnearFuego`)))

(event `SpawnearFuego`
  (params (StepID :type Name) (ActionTarget :type Name))
  (if (== ActionTarget (`self.TargetID`))
    (switch `name` StepID)))

(event `self.IsValidInteraction`
  (params (CanInteract :type Boolean))
  (if CanInteract
    (bind _asbp_player (cast `/Game/TestGame/Blueprints/BP_Player` (`GameplayStatics.GetPlayerCharacter` 0))
      (:`then`
        (`KismetSystemLibrary.PrintString` (`KismetSystemLibrary.GetDisplayName` _asbp_player))
        (`KismetSystemLibrary.PrintString` "Cast Ok")
        (if (`|EnumEquality` (`/Game/TestGame/Blueprints/BP_Player.CurrentElementState` _asbp_player) "NewEnumerator1")
          (message `/Game/TestGame/WidgetManager/BPI_ElementPickup.AgregarEnergia` _asbp_player 0.2 "NewEnumerator1")
          (`KismetSystemLibrary.PrintString` "Ya tienes el elemneto fuego")
          (`self.K2_DestroyActor`)
          (else
            (set `/Game/TestGame/Blueprints/BP_Player.TienePoderFuego` true _asbp_player)
            (set `/Game/TestGame/Blueprints/BP_Player.CurrentElementState` "NewEnumerator1" _asbp_player)
            (set `/Game/TestGame/Blueprints/BP_Player.HabilidadFuego` (+ 0.0 0.2) _asbp_player)
            (`KismetSystemLibrary.PrintString` "Desbloqueado")
            (`self.K2_DestroyActor`))))
      (:`CastFailed`
        (`KismetSystemLibrary.PrintString` "Cast Fallo")))))

(event `self.StartInteraction`)

(fn `UserConstructionScript`)
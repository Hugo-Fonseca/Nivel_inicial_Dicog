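; Interactive grille door that snaps its mesh between closed (zero rotation) and open (yawed a quarter turn).
; ToogleDoor sets the rotation instantly from IsOpen, then flips the flag; nothing in this Blueprint calls it.
; Interaction getters (type, hold duration, tap count, location) return only zero or first-enumerator values.
; The event graph is inactive, holding an unconnected copy of the toggle logic.
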(fn `GetHoldDuration`
  (returns (HoldDuration :type "Float (double-precision)"))
  (return 0.0))

(fn `GetInteractionLocation`
  (returns (Location :type "Vector Structure"))
  (return (0.0 0.0 0.0)))

(fn `GetInteractionType`
  (returns (`Interaction Type` :type "/Game/TestGame/InteractionSystem/E_InteractionType Enum"))
  (return "NewEnumerator0"))

(fn `GetTapCount`
  (returns (Value :type Integer))
  (return 0))

(fn `ToogleDoor`
  (bind _isopen (`self.IsOpen`))
  (if _isopen
    (`SceneComponent.K2_SetRelativeRotation` (`self.DoorMesh`) (`KismetMathLibrary.MakeRotator` 0.0) false false)
    (else
      (`SceneComponent.K2_SetRelativeRotation` (`self.DoorMesh`) (`KismetMathLibrary.MakeRotator` 0.0 0.0 90.0) false false)))
  (set `self.IsOpen` (not _isopen)))

(fn `UserConstructionScript`)
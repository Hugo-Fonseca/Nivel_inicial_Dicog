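; Interactive lever that triggers a referenced door when the player interacts with it.
; On Interact, it snaps the lever mesh to a tilted pitch and forwards an Interact message to DoorRef, with no animation or reset.
; Interaction query functions return the first interaction type and zeroed hold duration, tap count and location.
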(event `/Game/TestGame/InteractionSystem/BPI_Interactable.Interact`
  (params (Interactor :type "Actor Object Reference"))
  (`SceneComponent.K2_SetRelativeRotation` (`self.LeverMesh`) (`KismetMathLibrary.MakeRotator` 0.0 -45.0) false false)
  (message `/Game/TestGame/InteractionSystem/BPI_Interactable.Interact` (`self.DoorRef`) self))

(fn `GetHoldDuration`
  (returns (HoldDuration :type "Float (double-precision)"))
  (return 0.0))

(fn `GetInteractionLocation`
  (returns (Location :type "Vector Structure"))
  (return (0.0 0.0 0.0)))

(fn `GetInteractionType`
  (returns (`Interaction Type` :type "/Game/TestGame/InteractionSystem/E_InteractionType Enum"))
  (return "NewEnumerator0"))

(fn `GetTapCount`
  (returns (Value :type Integer))
  (return 0))

(fn `UserConstructionScript`)
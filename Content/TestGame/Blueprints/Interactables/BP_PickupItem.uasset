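; BP_PickupItem is an interactable pickup actor that destroys itself when Interact fires.
; Getter functions expose its interaction type, hold duration and tap count from variables, plus the world position of its InteractionLocation component.
; It contains no inventory or reward logic, and its construction script is empty.
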(event `self.Interact`
  (params (Interactor :type "Actor Object Reference"))
  (`self.K2_DestroyActor`))

(fn `GetHoldDuration`
  (returns (HoldDuration :type "Float (double-precision)"))
  (return (`self.Interaction Hold Duration`)))

(fn `GetInteractionLocation`
  (returns (Location :type "Vector Structure"))
  (return (`SceneComponent.K2_GetComponentLocation` (`self.InteractionLocation`))))

(fn `GetInteractionType`
  (returns (`Interaction Type` :type "/Game/TestGame/InteractionSystem/E_InteractionType Enum"))
  (return (`self.Interaction Type`)))

(fn `GetTapCount`
  (returns (Value :type Integer))
  (return (`self.Interaction Tap Count`)))

(fn `UserConstructionScript`)
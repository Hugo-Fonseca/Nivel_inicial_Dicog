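; BP_PuertaEnemies is an interactable door Blueprint whose Interact event is currently empty, so interacting with it does nothing.
; A disconnected graph fragment would toggle the DoorMesh yaw between closed and open using an IsOpen flag, but it never runs.
; The interaction getters return default values for type, hold duration, tap count and location.
; Despite the name, the graphs contain no enemy-related logic.
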(event `self.Interact`
  (params (Interactor :type "Actor Object Reference")))

(fn `GetHoldDuration`
  (returns (HoldDuration :type "Float (double-precision)"))
  (return 0.0))

(fn `GetInteractionLocation`
  (returns (Location :type "Vector Structure"))
  (return (0.0 0.0 0.0)))

(fn `GetInteractionType`
  (returns (`Interaction Type` :type "/Game/TestGame/InteractionSystem/E_InteractionType Enum"))
  (return "NewEnumerator0"))

(fn `GetTapCount`
  (returns (Value :type Integer))
  (return 0))

(fn `UserConstructionScript`)
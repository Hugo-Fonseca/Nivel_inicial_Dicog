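; Interactable lever that toggles a referenced gate door (DoorRef) each time it is used.
; Interact calls the door's toggle, flips IsActivated and snaps the lever mesh between tilted and default rotation, also sending InteractMessage to the door when switching off.
; A lock-on widget starts hidden and is shown or hidden through DisplayLockedonWidget.
; Interaction getters return fixed defaults, with zero hold duration, tap count and location.
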(event `self.ReceiveBeginPlay`
  (`SceneComponent.SetVisibility` (`self.LockOnWidget`) false false))

(event `self.Interact`
  (params (Interactor :type "Actor Object Reference"))
  (bind _isactivated (`self.IsActivated`))
  (`/Game/TestGame/Blueprints/Interactables/BP_PuertaInteractivaRejilla.ToogleDoor` (`self.DoorRef`))
  (if _isactivated
    (`SceneComponent.K2_SetRelativeRotation` (`self.LeverMesh`) (`KismetMathLibrary.MakeRotator` 0.0) false false)
    (message `/Game/TestGame/InteractionSystem/BPI_Interactable.Interact` (`self.DoorRef`) self)
    (else
      (`SceneComponent.K2_SetRelativeRotation` (`self.LeverMesh`) (`KismetMathLibrary.MakeRotator` 0.0 -45.0) false false)))
  (set `self.IsActivated` (not _isactivated)))

(event `self.DisplayLockedOnWidget`
  (params (ShowWidget :type Boolean))
  (`SceneComponent.SetVisibility` (`self.LockOnWidget`) ShowWidget false))

(fn `GetHoldDuration`
  (returns (HoldDuration :type "Float (double-precision)"))
  (return 0.0))

(fn `GetInteractionLocation`
  (returns (Location :type "Vector Structure"))
  (return (0.0 0.0 0.0)))

(fn `GetInteractionType`
  (returns (`Interaction Type` :type "/Game/TestGame/InteractionSystem/E_InteractionType Enum"))
  (return "NewEnumerator0"))

(fn `GetTapCount`
  (returns (Value :type Integer))
  (return 0))

(fn `UserConstructionScript`)
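; BP_Pared is an interactable wall that acts as a door driven by the game's progression events.
; On BeginPlay it binds a handler to the game instance's progression event.
; For Open Door or Close Door steps that pass an ActionTarget match, it calls ToggleVisibility on its static mesh.
; Both steps flip the current visibility, differing only in the propagate-to-children argument, and neither changes collision.
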(event `self.ReceiveBeginPlay`
  (add `/Game/TestGame/Games_Instance/BP_GamesInstance.OnProgressionEvent` (`/Game/ThirdPerson/Progresion/BFL_GameInstance.GetMyGameInstance`) (delegate `CustomEvent`)))

(event `CustomEvent`
  (params (StepID :type Name) (ActionTarget :type Name))
  (bind _staticmesh (`self.StaticMesh`))
  (bind _returnvalue (== ActionTarget (`self.Action Target`)))
  (switch `name` StepID
    (:`OpenDoor`
      (if _returnvalue
        (`SceneComponent.ToggleVisibility` _staticmesh false)))
    (:`CloseDoor`
      (if _returnvalue
        (`SceneComponent.ToggleVisibility` _staticmesh true)))))

(fn `UserConstructionScript`)